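; BP_Carter is a crater actor that tracks a DefaultPawn inside its box trigger, apparently intended to refill that player's oxygen.
; Box overlap events set MPlayer when the pawn enters and clear it when it leaves.
; While MPlayer is set, Tick prints the squared distance between the actor and the pawn.
; A French comment marks where the oxygen refill call belongs, but no such call exists yet.
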(event OnComponentBeginOverlap(Box)
  (params (OverlappedComponent :type Primitive%20Component%20Object%20Reference) (OtherActor :type Actor%20Object%20Reference) (OtherComp :type Primitive%20Component%20Object%20Reference) (OtherBodyIndex :type Integer) (bFromSweep :type Boolean) (SweepResult :type Hit%20Result%20Structure%20%28by%20ref%29))
  (bind _asdefault_pawn (Utilities|Casting|CastToDefaultPawn OtherActor))
  (Variables|Private|Setm_player _asdefault_pawn))

(event OnComponentEndOverlap(Box)
  (params (OverlappedComponent :type Primitive%20Component%20Object%20Reference) (OtherActor :type Actor%20Object%20Reference) (OtherComp :type Primitive%20Component%20Object%20Reference) (OtherBodyIndex :type Integer))
  (Utilities|Casting|CastToDefaultPawn OtherActor)
  (Variables|Private|Setm_player 0))

(event EventTick
  (params (DeltaSeconds :type Float%20%28single-precision%29))
  (if (!= (Variables|Private|Getm_player) 0)
    ;[1 1 1] Appelle de la fonction de remplissage de l'oxygène (calcul de distance au carré deja fait par le cratère)
    (Development|PrintString (Utilities|String|ToString(Float) (Class|KismetMathLibrary|VectorDistanceSquared (Transformation|GetActorLocation) (Transformation|GetActorLocation (Variables|Private|Getm_player)))) true true "(R=1.000000,G=0.282487,B=0.000000,A=1.000000)")))

(fn ConstructionScript)