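; Golgate is an enemy NPC that patrols a spline and lunges at the player when spotted.
; Tick sets or clears the target using a dot-product view cone and distance check, drawn as a debug cone.
; Timelines drive each phase: patrol, a force-feedback wind-up that reverts to patrol if sight is lost, then a lerped lunge to the player's captured position.
; When the lunge ends, it calls Death through a BP_PlayerController cast.
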(event Custom|AttackComportement
  (Components|Timeline|SetPlayRate (Variables|Default|GetAttackTimeline) 0.5)
  (bind _attacktimeline (Timeline|AttackTimeline PlayFromStart)
    (:Update
      (Utilities|IsValid (Variables|Private|Getm_player)
        (:Is%20Valid
          (Game|Feedback|PlayDynamicForceFeedback (Game|GetPlayerController 0) _attacktimeline 0.1 true true true true))
        (:Is%20Not%20Valid
          (CallFunction|PNJComportement)
          (Timeline|AttackTimeline Stop))))
    (:Finished
      (Variables|Private|Setm_currentPosition (Transformation|GetActorLocation))
      (Variables|Private|Setm_currentRotation (Transformation|GetActorRotation))
      (Variables|Private|Setm_targetPosition (Transformation|GetActorLocation (Variables|Private|Getm_player)))
      (Components|Timeline|SetPlayRate (Variables|Default|GetCrockTimeline) 3.0)
      (bind _crocktimeline (Timeline|CrockTimeline PlayFromStart)
        (:Update
          (Transformation|SetActorLocation (Math|Vector|Lerp(Vector) (Variables|Private|Getm_currentPosition) (Variables|Private|Getm_targetPosition) _crocktimeline) false false)
          (Transformation|SetActorRotation (Math|Rotator|Lerp(Rotator) (Variables|Private|Getm_currentRotation) (Math|Rotator|FindLookatRotation (Transformation|GetActorLocation) (Variables|Private|Getm_targetPosition)) _crocktimeline)))
        (:Finished
          (bind _asbp_player_controller (Utilities|Casting|CastToBP_PlayerController (Variables|Private|Getm_player)))
          (Default|Death _asbp_player_controller))))))

(event Custom|PNJComportement
  (bind _pnjcomportement (Timeline|PNJTimeline Play)
    (:Update
      (Utilities|IsValid (Variables|Private|Getm_player)
        (:Is%20Valid
          (CallFunction|AttackComportement)
          (Timeline|PNJTimeline Stop))
        (:Is%20Not%20Valid
          (Utilities|PNJMovement _pnjcomportement))))))

(event EventBeginPlay
  (Components|Timeline|SetPlayRate (Variables|Default|GetPNJTimeline) 0.01)
  (Variables|Private|Setm_player (Game|Player|GetPlayerPawn 0))
  (CallFunction|PNJComportement))

(event EventTick
  (params (DeltaSeconds :type Float%20%28single-precision%29))
  (bind _fiealdofview (Variables|Public|GetFiealdOfView))
  (Utilities|FlowControl|Sequence
    (:then_0
      (if (and (>= (Math|Vector|DotProduct (Math|Vector|Normalize (- (Transformation|GetActorLocation (Game|Player|GetPlayerPawn 0)) (Transformation|GetWorldLocation (Variables|Default|GetPivot))) 0.0) (Math|Vector|GetForwardVector (Variables|Default|GetPivot))) (Math|Trig|Cos(Radians) (Math|Trig|DegreesToRadians (* (Variables|Public|GetFiealdOfView) 0.5)))) (<= (Math|Vector|Distance(Vector) (Transformation|GetActorLocation (Game|Player|GetPlayerPawn 0)) (Transformation|GetWorldLocation (Variables|Default|GetPivot))) (Variables|Public|GetMaxDistance)))
        (Variables|Private|Setm_player (Game|Player|GetPlayerPawn 0))
        (else
          (Variables|Private|Setm_player 0))))
    (:then_1
      (Class|KismetSystemLibrary|DrawDebugConeinDegrees (Transformation|GetWorldLocation (Variables|Default|GetPivot)) (Math|Vector|GetForwardVector (Variables|Default|GetPivot)) (Variables|Public|GetMaxDistance) _fiealdofview _fiealdofview 12 "(R=1.000000,G=1.000000,B=1.000000,A=1.000000)" 0.0 0.0))))

(fn ConstructionScript
  (Actor|GetAllActorswithTag "Checkpoint"))