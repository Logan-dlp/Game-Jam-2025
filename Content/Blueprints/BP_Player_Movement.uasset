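; BP_Player_Movement is a player Blueprint that moves the actor on the X/Z plane from 2D input.
; BeginPlay registers the Player_Controler mapping context with the Enhanced Input subsystem of player 0.
; The Move action scales its input by Speed and line-traces from the actor's location to the target against WorldStatic and WorldDynamic objects.
; The actor jumps to the target without sweep only when nothing is hit, with no delta-time scaling.
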(event Input|EnhancedActionEvents|EnhancedInputActionMove
  (params (ActionValue :type Vector%202D%20Structure) (ElapsedSeconds :type Float%20%28double-precision%29) (TriggeredSeconds :type Float%20%28double-precision%29) (InputAction :type Input%20Action%20Object%20Reference :default "/Game/Blueprints/Move.Move"))
  (bind _returnvalue (Transformation|GetActorLocation))
  (bind _speed (Variables|Default|GetSpeed))
  ;[1 1 1] Movement
  (bind _output_get (Variables|Default|SetVectorInputResult ActionValue))
  (bind _returnvalue_2 (Collision|LineTraceForObjects _returnvalue (+ _returnvalue (Math|Vector|MakeVector (.x (* _output_get (Variables|Default|GetSpeed))) 0.0 (.y (* _output_get (Variables|Default|GetSpeed))))) (Utilities|Array|MakeArray "ObjectTypeQuery2" "ObjectTypeQuery1") false 0 "None"))
  (if (not _returnvalue_2)
    (Transformation|SetActorLocation (+ (Transformation|GetActorLocation) (Math|Vector|MakeVector (* (.x (Variables|Default|GetVectorInputResult)) _speed) 0.0 (* (.y (Variables|Default|GetVectorInputResult)) _speed))) false false)))

(event EventBeginPlay
  ;[1 1 1] Appel du controler
  (bind _asplayer_controller (Utilities|Casting|CastToPlayerController (Game|GetPlayerController 0)))
  (Utilities|IsValid (PlayerController|LocalPlayerSubsystems|GetEnhancedInputLocalPlayerSubsystem _asplayer_controller)
    (:Is%20Valid
      (Input|AddMappingContext (PlayerController|LocalPlayerSubsystems|GetEnhancedInputLocalPlayerSubsystem _asplayer_controller) "/Game/Blueprints/Player_Controler.Player_Controler" 0 "(bIgnoreAllPressedKeysUntilRelease=True,bForceImmediately=False,bNotifyUserSettings=False)"))))

(event Collision|EventActorBeginOverlap
  (params (OtherActor :type Actor%20Object%20Reference)))

(fn ConstructionScript)