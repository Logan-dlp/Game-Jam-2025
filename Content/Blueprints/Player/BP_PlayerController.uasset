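; Player blueprint that moves on the X/Z plane, frees caged fish and manages an oxygen bubble.
; Enhanced Input drives swept movement and interaction with the fish cage found by a per-tick sphere trace.
; The bubble's scale acts as oxygen: it shrinks each tick, grows through RechargeBubule and feeds a percentage text.
; At zero percent, Death opens the game over level.
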(event Custom|RechargeBubule
  (params (Distance :type Float%20%28double-precision%29))
  (bind _bubule (Variables|Default|GetBubule))
  (bind _bubulescalemax (Variables|Public|GetBubuleScaleMax))
  (bind _rechargespeed (Variables|Public|GetRechargeSpeed))
  (bind _returnvalue (Transformation|GetWorldScale _bubule))
  (bind _returnvalue_2 (* Distance _rechargespeed))
  (bind _returnvalue_3 (+ _returnvalue _returnvalue_2))
  (if (CallFunction|<=Vector _returnvalue_3 (Math|Vector|MakeVector _bubulescalemax _bubulescalemax _bubulescalemax))
    (Transformation|SetRelativeScale3D (Variables|Default|GetBubule) _returnvalue_3)))

(event Custom|Death
  (Development|PrintString "Hello")
  (Game|OpenLevel(byName) "ST_Game_Over"))

(event Input|EnhancedActionEvents|EnhancedInputActionMove
  (params (ActionValue :type Vector%202D%20Structure) (ElapsedSeconds :type Float%20%28double-precision%29) (TriggeredSeconds :type Float%20%28double-precision%29) (InputAction :type Input%20Action%20Object%20Reference :default "/Game/Inputs/Move.Move"))
  (bind _m_speed (Variables|Private|Getm_speed))
  (bind _m_speed_2 (Variables|Private|Getm_speed))
  (bind _returnvalue (* ActionValue _m_speed))
  ;[1 1 1] Movement
  (Transformation|SetActorLocation (+ (Transformation|GetActorLocation) (Math|Vector|MakeVector (* (.x _returnvalue) _m_speed_2) 0.0 (* (.y _returnvalue) _m_speed_2))) true false))

(event Input|EnhancedActionEvents|EnhancedInputActionInteraction
  (params (ActionValue :type Boolean) (ElapsedSeconds :type Float%20%28double-precision%29) (TriggeredSeconds :type Float%20%28double-precision%29) (InputAction :type Input%20Action%20Object%20Reference :default "/Game/Inputs/Interaction.Interaction"))
  ;[1 1 1] Interact
  (:Started
    (Utilities|IsValid (Variables|Private|Getm_currentFishCage)
      (:Is%20Valid
        (Default|FreeFish (Variables|Private|Getm_currentFishCage) self)))))

(event EventBeginPlay
  (bind _returnvalue (Game|GetPlayerController 0))
  (bind _bubulescalemax (Variables|Public|GetBubuleScaleMax))
  (bind _returnvalue_2 (PlayerController|LocalPlayerSubsystems|GetEnhancedInputLocalPlayerSubsystem _returnvalue))
  ;[1 1 1] Appel du controler
  (Utilities|IsValid _returnvalue_2
    (:Is%20Valid
      (Input|AddMappingContext _returnvalue_2 "/Game/Inputs/Player_Input.Player_Input" 0 "(bIgnoreAllPressedKeysUntilRelease=True,bForceImmediately=False,bNotifyUserSettings=False)")
      (Transformation|SetRelativeScale3D (Variables|Default|GetBubule) (Math|Vector|MakeVector _bubulescalemax _bubulescalemax _bubulescalemax)))))

(event EventTick
  (params (DeltaSeconds :type Float%20%28single-precision%29))
  (bind _returnvalue (Transformation|GetActorLocation))
  (bind _bubule (Variables|Default|GetBubule))
  (bind _bubule_2 (Variables|Default|GetBubule))
  (bind _bubulescalemin (Variables|Public|GetBubuleScaleMin))
  (bind _bubulescalemin_2 (Variables|Public|GetBubuleScaleMin))
  (bind _bubulescalemin_3 (Variables|Public|GetBubuleScaleMin))
  (bind _dechargespeed (Variables|Public|GetDechargeSpeed))
  (bind _bubulescalemax (Variables|Public|GetBubuleScaleMax))
  (bind _returnvalue_2 (Transformation|GetWorldScale _bubule))
  (bind _returnvalue_3 (Transformation|GetWorldScale _bubule_2))
  (bind _returnvalue_4 (Math|Vector|MakeVector _bubulescalemax _bubulescalemax _bubulescalemax))
  (bind _returnvalue_5 (Math|Vector|MakeVector _bubulescalemin_3 _bubulescalemin_3 _bubulescalemin_3))
  (bind _returnvalue_6 (Math|Vector|MakeVector _bubulescalemin_2 _bubulescalemin_2 _bubulescalemin_2))
  (bind _returnvalue_7 (Math|Vector|VectorLength _returnvalue_2))
  (bind _returnvalue_8 (Math|Vector|VectorLength _returnvalue_6))
  (bind _returnvalue_9 (Math|Vector|VectorLength _returnvalue_4))
  (bind _returnvalue_10 (Math|Vector|VectorLength _returnvalue_5))
  (bind _returnvalue_11 (- _returnvalue_3 _dechargespeed))
  (bind _returnvalue_12 (- _returnvalue_7 _returnvalue_8))
  (bind _returnvalue_13 (- _returnvalue_9 _returnvalue_10))
  (bind _returnvalue_14 (/ _returnvalue_12 _returnvalue_13))
  (bind _returnvalue_15 (* _returnvalue_14 1e+02))
  (bind _returnvalue_16 (Class|KismetMathLibrary|FTrunc64 _returnvalue_15))
  (Utilities|FlowControl|Sequence
    (:then_0
      ;[1 1 1] Free Fish
      (bind _outhit (Collision|SphereTraceForObjects _returnvalue _returnvalue 2e+02 (Utilities|Array|MakeArray "ObjectTypeQuery1" "ObjectTypeQuery2") false 0 "ForOneFrame"))
      (bind _asbp_fish_cage (Utilities|Casting|CastToBP_FishCage (.HitActor (Collision|BreakHitResult _outhit)))
        (:then
          (bind _output_get (Variables|Private|Setm_currentFishCage _asbp_fish_cage))
          (Default|Interaction _output_get "NewEnumerator1"))
        (:CastFailed
          (Utilities|IsValid (Variables|Private|Getm_currentFishCage)
            (:Is%20Valid
              (Default|Interaction (Variables|Private|Getm_currentFishCage) "NewEnumerator0"))
            (:Is%20Not%20Valid
              _))
          (Variables|Private|Setm_currentFishCage 0))))
    (:then_1
      (if (CallFunction|>=Vector _returnvalue_11 (Math|Vector|MakeVector _bubulescalemin _bubulescalemin _bubulescalemin))
        (Transformation|SetRelativeScale3D _bubule_2 _returnvalue_11)
        (else
          (Rendering|SetVisibility (Variables|Default|GetBubule) false false))))
    (:then_2
      (Rendering|Components|TextRender|SetText (Variables|Default|Getoxy) (Utilities|Text|FormatText "{p} %" _returnvalue_16))
      (if (<= _returnvalue_16 0)
        (Utilities|FlowControl|DoOnce false
          (:Completed
            (CallFunction|Death)))))))

(fn ConstructionScript)

(fn >=Vector
  (params (vect%20a :type Vector) (vect%20b :type Vector))
  (bind (_x _y _z) (Math|Vector|BreakVector vect%20a))
  (bind (_x_2 _y_2 _z_2) (Math|Vector|BreakVector vect%20b))
  (return (Math|Boolean|ANDBoolean (>= _x _x_2) (>= _y _y_2) (>= _z _z_2))))

(fn <=Vector
  (params (vect%20a :type Vector) (vect%20b :type Vector))
  (bind (_x _y _z) (Math|Vector|BreakVector vect%20a))
  (bind (_x_2 _y_2 _z_2) (Math|Vector|BreakVector vect%20b))
  (return (Math|Boolean|ANDBoolean (<= _x _x_2) (<= _y _y_2) (<= _z _z_2))))