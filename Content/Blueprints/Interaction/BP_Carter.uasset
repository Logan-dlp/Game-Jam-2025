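; BP_Carter is an interaction actor that recharges the player's "Bubule" while the player is inside its box trigger.
; Box overlap events store the entering BP_PlayerController actor and clear it on exit.
; While that reference is valid, Tick passes the distance between the Pivot component and the player to RechargeBubule every frame, leaving the recharge logic to the player.
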(event OnComponentBeginOverlap(Box)
  (params (OverlappedComponent :type Primitive%20Component%20Object%20Reference) (OtherActor :type Actor%20Object%20Reference) (OtherComp :type Primitive%20Component%20Object%20Reference) (OtherBodyIndex :type Integer) (bFromSweep :type Boolean) (SweepResult :type Hit%20Result%20Structure%20%28by%20ref%29))
  (bind _asbp_player_controller (Utilities|Casting|CastToBP_PlayerController OtherActor))
  (Variables|Private|Setm_player _asbp_player_controller))

(event OnComponentEndOverlap(Box)
  (params (OverlappedComponent :type Primitive%20Component%20Object%20Reference) (OtherActor :type Actor%20Object%20Reference) (OtherComp :type Primitive%20Component%20Object%20Reference) (OtherBodyIndex :type Integer))
  (Utilities|Casting|CastToBP_PlayerController OtherActor)
  (Variables|Private|Setm_player 0))

(event EventTick
  (params (DeltaSeconds :type Float%20%28single-precision%29))
  (Utilities|IsValid (Variables|Private|Getm_player)
    (:Is%20Valid
      (Default|RechargeBubule (Variables|Private|Getm_player) (Math|Vector|Distance(Vector) (Transformation|GetWorldLocation (Variables|Default|GetPivot)) (Transformation|GetActorLocation (Variables|Private|Getm_player)))))))

(fn ConstructionScript)